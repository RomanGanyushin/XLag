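; Day-night cycle actor that tracks a day count and time of day while animating the sun and sky.
; The SunMovement timeline, rate-scaled by DaySpeed, increments Day and restarts whenever it finishes.
; Each tick builds a Timespan from it and applies its curves to sun rotation and sun and skylight intensity, then refreshes the sky sphere.
; SetNewTime jumps to a given Timespan by converting it to decimal hours.
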(event EventBeginPlay
  (bind (_direction _ysunpitch _zsuncurve _time _skylightintencity _sunlightintencity) (Timeline|SunMovement SetNewTime)
    (:Finished
      (CallFunction|DayTickSys)
      (Timeline|SunMovement PlayFromStart))))

(event EventTick
  (params (DeltaSeconds :type Float%20%28single-precision%29))
  (CallFunction|TimeSystem)
  (Variables|Default|SetMovementSec (stale EventBeginPlay _time))
  (Transformation|SetActorRotation (Variables|Default|GetSunLight) (Math|Rotator|MakeRotator 0.0 (stale EventBeginPlay _ysunpitch) (stale EventBeginPlay _zsuncurve)))
  (Rendering|Components|Light|SetIntensity (Variables|/Script/Engine.SkyLight|GetLightComponent (Variables|Default|GetSkyLight)) (stale EventBeginPlay _skylightintencity))
  (Rendering|Components|Light|SetIntensity (Variables|/Script/Engine.Light|GetLightComponent (Variables|Default|GetSunLight)) (stale EventBeginPlay _sunlightintencity))
  (Default|UpdateSunDirection (Variables|Default|GetSkySphereBP)))

(fn ConstructionScript
  (Components|Timeline|SetPlayRate (Variables|Default|GetSunMovement) (Variables|Default|GetDaySpeed)))

(fn TimeSystem
  (bind _output_get (Variables|Default|SetTime (Math|Timespan|MakeTimespan (Variables|Default|GetDay) 0 0 (Math|Float|Truncate (Variables|Default|GetMovementSec))))))

(fn DayTickSys
  (Variables|Default|SetDay (+ (Variables|Default|GetDay) 1))
  (return))

(fn SetNewTime
  (params (Time :type Timespan%20Structure))
  (bind (_days _hours _minutes _seconds) (Math|Timespan|BreakTimespan Time))
  (Variables|Default|SetDay _days)
  (Components|Timeline|SetNewTime (Variables|Default|GetSunMovement) (CallFunction|ConvertTimeinDeC _hours _minutes _seconds)))

(fn ConvertTimeinDeC
  (params (Hours :type Integer) (Min :type Integer) (Sec :type Integer))
  (return (+ (Math|Conversions|ToFloat(Integer) Hours) (/ (+ (Math|Conversions|ToFloat(Integer) Min) (/ (Math|Conversions|ToFloat(Integer) Sec) 6e+01)) 6e+01))))