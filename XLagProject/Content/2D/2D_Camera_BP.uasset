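; Top-down strategy camera with arm zoom, axis and screen-edge panning, which also turns mouse input into worker orders.
; Left-drag traces world corners into BP_OperationSelection; on release, the UI's operation type picks the BP_TaskManager task.
; Building mode moves a BP_BuildingManager preview under the cursor and creates a build task on release.
; Manager references are found in the construction script; mouse-rotation gate toggles are unwired.
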(event Custom|OnCreateMiningTask
  (Class|XLagTaskManager|CreateExtractMineralTask (Variables|References|GetBP_TaskManagerRef) (Variables|References|GetBP_OperationSelRef) (Utilities|Array|Get(acopy) (Variables|/Script/XLagProject.XLagMineralManager|GetMineralDescCollection (Variables|References|GetBP_MineralManagerRef)) (Class|ComboBoxString|GetSelectedIndex (Variables|/Game/UI/2D/2D_Select_Mining_WB.2D_Select_Mining_WB_C|GetComboBoxString_135 (Variables|/Game/UI/2D/2D_Main_WB.2D_Main_WB_C|Get2D_Select_Mining_WB (Variables|/Game/UI/2D/2D_Select_WB.2D_Select_WB_C|Get2DMainRef (Variables|References|Get2D_SelectWBRef))))))))

(event Custom|OnCreateAlignTask
  (Class|XLagTaskManager|CreateGroundAlignTask (Variables|References|GetBP_TaskManagerRef) (Variables|References|GetBP_OperationSelRef) "Diging" "GraundGrass" 1e+02))

(event Custom|OnCreateSearchingTask
  (Class|XLagTaskManager|CreateSearchMineralTask (Variables|References|GetBP_TaskManagerRef) (Variables|References|GetBP_OperationSelRef) (Utilities|Array|Get(acopy) (Class|XLagMineralManager|GetSearchableMineralDescCollection (Variables|References|GetBP_MineralManagerRef)))))

(event Custom|OnCreateCuttingTask
  (Class|XLagTaskManager|CreateCuttingTreeTask (Variables|References|GetBP_TaskManagerRef) (Variables|References|GetBP_OperationSelRef)))

(event Custom|OnCreateCroplandTask
  (Class|XLagTaskManager|CreateCroplandTask (Variables|References|GetBP_TaskManagerRef) (Variables|References|GetBP_OperationSelRef)))

(event Custom|OnCreateCultivateTask
  (Class|XLagTaskManager|CreateCultivationTask (Variables|References|GetBP_TaskManagerRef) (Variables|References|GetBP_OperationSelRef) (Utilities|Array|Get(acopy) (Variables|/Script/XLagProject.XLagCropManager|GetCropDescCollection (Variables|References|GetBP_CropManagerRef)))))

(event Custom|OnCreateProductionTask
  (Class|XLagTaskManager|CreateProductionTask (Variables|References|GetBP_TaskManagerRef) (Utilities|Array|Get(acopy) (Variables|/Script/XLagProject.XLagProductionSchemasManager|GetProductionSchemaCollection (Variables|References|GetBP_ProdSchemasManagerRef)) (Class|ComboBoxString|GetSelectedIndex (Variables|/Game/UI/2D/2D_Select_Production_WB.2D_Select_Production_WB_C|GetComboBoxString_135 (Variables|/Game/UI/2D/2D_Main_WB.2D_Main_WB_C|Get2D_Select_Production_WB (Variables|/Game/UI/2D/2D_Select_WB.2D_Select_WB_C|Get2DMainRef (Variables|References|Get2D_SelectWBRef)))))) (Variables|References|GetBP_OperationSelRef) 1e+02))

(event Input|ActionEvents|InputActionPan
  (params (Key :type Key%20Structure :default "None"))
  ;[1 1 1] Поворот Y
)

(event Input|ActionEvents|InputActionZoomOut
  (params (Key :type Key%20Structure :default "None"))
  (bind _springarm (Variables|Default|GetSpringArm))
  ;[1 1 1] Масштаб камеры
  (:Pressed
    (Variables|/Script/Engine.SpringArmComponent|SetTargetArmLength _springarm (Math|Float|Clamp(Float) (+ (Variables|/Script/Engine.SpringArmComponent|GetTargetArmLength _springarm) (Variables|CameraMove|GetCameraArmSpeed)) (Variables|CameraMove|GetMinArmLength) (Variables|CameraMove|GetMaxArmLength)))))

(event Input|ActionEvents|InputActionZoomIn
  (params (Key :type Key%20Structure :default "None"))
  (bind _springarm (Variables|Default|GetSpringArm))
  ;[1 1 1] Масштаб камеры
  (:Pressed
    (Variables|/Script/Engine.SpringArmComponent|SetTargetArmLength _springarm (Math|Float|Clamp(Float) (- (Variables|/Script/Engine.SpringArmComponent|GetTargetArmLength _springarm) (Variables|CameraMove|GetCameraArmSpeed)) (Variables|CameraMove|GetMinArmLength) (Variables|CameraMove|GetMaxArmLength)))))

(event Input|ActionEvents|InputActionPan
  (params (Key :type Key%20Structure :default "None"))
  ;[1 1 1] Поворот камеры Х
)

(event Input|AxisEvents|InputAxisMoveForward
  (params (AxisValue :type Float%20%28single-precision%29))
  ;[1 1 1] Перемещение по Х
  (if (not (Variables|CameraMove|GetDisableCamNav))
    (Transformation|SetActorTransform (Utilities|MovementX (CallFunction|MovementSpeedCalculation) (Variables|CameraMove|GetFastMoveMultiplier) AxisValue))))

(event Input|AxisEvents|InputAxisMoveRight
  (params (AxisValue :type Float%20%28single-precision%29))
  ;[1 1 1] Перемещение по Y
  (if (not (Variables|CameraMove|GetDisableCamNav))
    (Transformation|SetActorTransform (Utilities|MovementY AxisValue (CallFunction|MovementSpeedCalculation) (Variables|CameraMove|GetFastMoveMultiplier)))))

(event Input|MouseEvents|MouseX
  (params (AxisValue :type Float%20%28single-precision%29))
  (bind _returnvalue (Transformation|GetActorRotation))
  (bind (_roll _pitch _yaw) (Math|Rotator|BreakRotator _returnvalue))
  ;[1 1 1] Поворот камеры Х
  (Utilities|FlowControl|Gate true
    (:Exit
      (Transformation|SetActorRotation (Math|Rotator|MakeRotator _roll (+ _pitch (* AxisValue (Variables|CameraMove|GetPanSensitivity))) _yaw)))))

(event Input|MouseEvents|MouseY
  (params (AxisValue :type Float%20%28single-precision%29))
  (bind _returnvalue (Transformation|GetActorRotation))
  (bind (_roll _pitch _yaw) (Math|Rotator|BreakRotator _returnvalue))
  ;[1 1 1] Поворот Y
  (Utilities|FlowControl|Gate true
    (:Exit
      (Transformation|SetActorRotation (Math|Rotator|MakeRotator (+ _roll (* AxisValue (Variables|CameraMove|GetPanSensitivity))) _pitch _yaw)))))

(event Input|MouseEvents|MouseY
  (params (AxisValue :type Float%20%28single-precision%29))
  (bind _returnvalue (Game|GetPlayerController 0))
  (bind _hitresult (Game|Player|GetHitResultUnderCursorbyChannel _returnvalue "TraceTypeQuery2" true))
  (bind _location (Collision|BreakHitResult _hitresult))
  ;[1 1 1] Строительство
  (if (Variables|Buttons|GetBuildingButtonPressed)
    (Class|XLagBuildingManager|SetPreviewPosition (Variables|References|GetBP_BuildingManagerRef) (.x _location) (.y _location))))

(event Input|MouseEvents|MouseX
  (params (AxisValue :type Float%20%28single-precision%29))
  ;[1 1 1] скроллинг мышью по краям
  (if (not (Variables|CameraMove|GetDisableCamNav))
    (bind (_deltaxspeed _deltayspeed) (Utilities|ScreenEdgeMovement))
    (Transformation|AddActorLocalOffset (Math|Vector|MakeVector _deltaxspeed _deltayspeed 0.0) true false)))

(event Input|MouseEvents|MouseY
  (params (AxisValue :type Float%20%28single-precision%29))
  ;[1 1 1] скроллинг мышью по краям
  (if (not (Variables|CameraMove|GetDisableCamNav))
    (Utilities|ScreenEdgeMovement) ; enters at MouseY
  ))

(event Input|MouseEvents|MouseY
  (params (AxisValue :type Float%20%28single-precision%29))
  (bind _returnvalue (Game|GetPlayerController 0))
  (bind _hitresult (Game|Player|GetHitResultUnderCursorbyChannel _returnvalue "TraceTypeQuery2" true))
  (bind _location (Collision|BreakHitResult _hitresult))
  ;[1 1 1] Выделение площади
  (if (!= (Variables|/Game/UI/2D/2D_Select_WB.2D_Select_WB_C|GetOperationType (Variables|References|Get2D_SelectWBRef)) 0)
    (Utilities|FlowControl|Gate true
      (:Exit
        (Class|XLagSelectComponent|SetSecondWorldPoint (Variables|References|GetBP_OperationSelRef) (.x _location) (.y _location))))))

(event Input|MouseEvents|MouseX
  (params (AxisValue :type Float%20%28single-precision%29))
  (bind _returnvalue (Game|GetPlayerController 0))
  (bind _hitresult (Game|Player|GetHitResultUnderCursorbyChannel _returnvalue "TraceTypeQuery2" true))
  (bind _location (Collision|BreakHitResult _hitresult))
  ;[1 1 1] Выделение площади
  (if (!= (Variables|/Game/UI/2D/2D_Select_WB.2D_Select_WB_C|GetOperationType (Variables|References|Get2D_SelectWBRef)) 0)
    (Utilities|FlowControl|Gate true
      (:Exit
        (Class|XLagSelectComponent|SetSecondWorldPoint (Variables|References|GetBP_OperationSelRef) (.x _location) (.y _location))))))

(event Input|MouseEvents|MouseX
  (params (AxisValue :type Float%20%28single-precision%29))
  (bind _returnvalue (Game|GetPlayerController 0))
  (bind _hitresult (Game|Player|GetHitResultUnderCursorbyChannel _returnvalue "TraceTypeQuery2" true))
  (bind _location (Collision|BreakHitResult _hitresult))
  ;[1 1 1] Строительство
  (if (Variables|Buttons|GetBuildingButtonPressed)
    (Class|XLagBuildingManager|SetPreviewPosition (Variables|References|GetBP_BuildingManagerRef) (.x _location) (.y _location))))

(event Input|MouseEvents|LeftMouseButton
  (params (Key :type Key%20Structure :default "None"))
  (bind _returnvalue (Game|GetPlayerController 0))
  (bind _2d_selectwbref (Variables|References|Get2D_SelectWBRef))
  (bind _hitresult (Game|Player|GetHitResultUnderCursorbyChannel _returnvalue "TraceTypeQuery2" true))
  (bind _location (Collision|BreakHitResult _hitresult))
  ;[1 1 1] Выделение площади
  (:Pressed
    (if (!= (Variables|/Game/UI/2D/2D_Select_WB.2D_Select_WB_C|GetOperationType (Variables|References|Get2D_SelectWBRef)) 0)
      (Class|XLagSelectComponent|SetFirstWorldPoint (Variables|References|GetBP_OperationSelRef) (.x _location) (.y _location))))
  (:Released
    (switch Utilities|FlowControl|Switch|SwitchonSelectType_EN (Variables|/Game/UI/2D/2D_Select_WB.2D_Select_WB_C|GetOperationType (Variables|References|Get2D_SelectWBRef))
      (:NewEnumerator0
        (CallFunction|OnCreateAlignTask))
      (:NewEnumerator4
        (CallFunction|OnCreateSearchingTask))
      (:NewEnumerator1
        (CallFunction|OnCreateCuttingTask))
      (:NewEnumerator2
        (CallFunction|OnCreateMiningTask))
      (:NewEnumerator5
        (CallFunction|OnCreateCroplandTask))
      (:NewEnumerator6
        (CallFunction|OnCreateCultivateTask))
      (:NewEnumerator7
        (CallFunction|OnCreateProductionTask)))
    (Variables|/Game/UI/2D/2D_Select_WB.2D_Select_WB_C|SetOperationType _2d_selectwbref "NewEnumerator3")
    (Default|OnOperationTypeChanged _2d_selectwbref)))

(event Input|MouseEvents|LeftMouseButton
  (params (Key :type Key%20Structure :default "None"))
  (bind _returnvalue (Game|GetPlayerController 0))
  (bind _hitresult (Game|Player|GetHitResultUnderCursorbyChannel _returnvalue "TraceTypeQuery2" true))
  (bind _location (Collision|BreakHitResult _hitresult))
  ;[1 1 1] Выделение площади
  (:Pressed
    (if (!= (Variables|/Game/UI/2D/2D_Select_WB.2D_Select_WB_C|GetOperationType (Variables|References|Get2D_SelectWBRef)) 0)
      (Utilities|FlowControl|Gate true) ; enters at Open
    ))
  (:Released
    (Utilities|FlowControl|Gate true) ; enters at Close
  ))

(event Input|MouseEvents|LeftMouseButton
  (params (Key :type Key%20Structure :default "None"))
  ;[1 1 1] Строительство
  (:Released
    (if (Variables|Buttons|GetBuildingButtonPressed)
      (Class|XLagTaskManager|CreateBuildingTask (Variables|References|GetBP_TaskManagerRef) (Variables|/Script/XLagProject.XLagBuildingManager|GetSelectBuilding (Variables|References|GetBP_BuildingManagerRef)))
      (Variables|/Script/XLagProject.XLagBuildingManager|SetPreviewSelectBuilding (Variables|References|GetBP_BuildingManagerRef) false)
      (Variables|Buttons|SetBuildingButtonPressed false)
      (Class|Button|SetBackgroundColor (Variables|/Game/UI/2D/2D_Build_WB.2D_Build_WB_C|GetButton_171 (Variables|References|Get2D_BuildWBRef)) "(R=1.000000,G=1.000000,B=1.000000,A=1.000000)"))))

(fn ConstructionScript
  (bind _returnvalue (Actor|GetActorOfClass "/Game/Selection/BP_OperationSelection.BP_OperationSelection_C"))
  (Variables|References|SetBP_OperationSelRef _returnvalue)
  (bind _returnvalue_2 (Actor|GetActorOfClass "/Game/NPCs/Tasks/BP_TaskManager.BP_TaskManager_C"))
  (Variables|References|SetBP_TaskManagerRef _returnvalue_2)
  (bind _returnvalue_3 (Actor|GetActorOfClass "/Game/Buildings/BP_BuildingManager.BP_BuildingManager_C"))
  (Variables|References|SetBP_BuildingManagerRef _returnvalue_3)
  (bind _returnvalue_4 (Actor|GetActorOfClass "/Game/Minerals/BP_MineralManager.BP_MineralManager_C"))
  (Variables|References|SetBP_MineralManagerRef _returnvalue_4)
  (bind _returnvalue_5 (Actor|GetActorOfClass "/Game/Crops/BP_CropsManager.BP_CropsManager_C"))
  (Variables|References|SetBP_CropManagerRef _returnvalue_5)
  (bind _returnvalue_6 (Actor|GetActorOfClass "/Game/Production/BP_ProdSchemasManager.BP_ProdSchemasManager_C"))
  (Variables|References|SetBP_ProdSchemasManagerRef _returnvalue_6))

(fn MovementSpeedCalculation
  (return (Math|Float|Clamp(Float) (/ (Variables|/Script/Engine.SpringArmComponent|GetTargetArmLength (Variables|Default|GetSpringArm)) 1e+02) 5.0 2e+01)))