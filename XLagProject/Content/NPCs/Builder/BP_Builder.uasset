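; BP_Builder is a builder NPC that carries a shovel mesh and has a digging flag.
; On BeginPlay, when digging is set, it attaches the shovel mesh to the Shovel component with relative transform rules.
; Every tick, regardless of that flag, it snaps the shovel to one skeletal mesh socket, aims it along the direction to a second socket, and applies a fixed local rotation offset.
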(event EventBeginPlay
  (if (Variables|Default|GetIsDiging)
    (Transformation|AttachComponentToComponent (Variables|Default|GetShovelMeshComp) (Variables|Default|GetShovel) "None" "KeepRelative" "KeepRelative" "KeepRelative" true)))

(event EventTick
  (params (DeltaSeconds :type Float%20%28single-precision%29))
  (bind _mesh (Variables|Character|GetMesh))
  (bind _shovelmeshcomp (Variables|Default|GetShovelMeshComp))
  (bind _returnvalue (Transformation|GetSocketLocation _mesh "ShovelSocket"))
  ;[1 1 1] Ориентация лопаты
  (Transformation|SetWorldLocationAndRotation _shovelmeshcomp _returnvalue (Class|KismetMathLibrary|QuatRotator (Class|KismetMathLibrary|ToQuaterion(Vector) (- (Transformation|GetSocketLocation _mesh "ShovelSocket2") _returnvalue))) false false)
  (Transformation|AddLocalRotation _shovelmeshcomp "-90.000000, 0,-0.000000" false false))

(fn ConstructionScript)