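; BP_Tools_Component is an NPC component for attaching a tool actor to the character's mesh.
; ToolADD casts the input to BP_Tools_Actor and, behind a not-valid check on Tool, stores it and calls ToolAttach.
; ToolAttach parents the tool to a named socket on the character mesh using keep-relative rules.
; Init extends the parent with a debug print, but its EventGraph call is never executed.
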(fn -Init
  (|CallParentFunction)
  (Development|PrintString "Hello"))

(fn ToolADD
  (params (Tool :type BP%20Tools%20Actor%20Object%20Reference) (SocketName :type Name))
  (bind _asbp_tools_actor (Utilities|Casting|CastToBP_Tools_Actor Tool))
  (Variables|Default|GetTool
    (:then)
    (:else
      (bind _output_get (Variables|Default|SetTool _asbp_tools_actor))
      (CallFunction|ToolAttach _output_get SocketName))))

(fn ToolAttach
  (params (Weapon :type BP%20Tools%20Actor%20Object%20Reference) (SocketName :type Name))
  (Transformation|AttachComponentToComponent Weapon (Variables|/Script/Engine.Character|GetMesh (Variables|Default|GetCharacter)) SocketName "KeepRelative" "KeepRelative" "KeepRelative" true))